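; BP_Exhibitor is an exhibit room that displays a center object through switchable corner cameras.
; The construction script scales and places six box faces from Length, Width and Height, applies one material and centers the object vertically with an offset.
; BeginPlay spawns a BP_CameraPawn aimed at the object, currently at one bottom corner unless OnlyTop.
; Functions cycle the Cameras array, unpopulated here, toggle layers by four-index offsets, and adjust FOV.
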(event EventBeginPlay
  (CallFunction|SpawnCamsAlongCorners))

(event Collision|EventActorBeginOverlap
  (params (OtherActor :type Actor%20Object%20Reference)))

(event EventTick
  (params (DeltaSeconds :type Float%20%28single-precision%29)))

(event EventChangeZoom
  (params (Value :type Float%20%28single-precision%29))
  (Camera|SetFieldOfView (+ Value 0.0)))

(fn ConstructionScript
  (Utilities|FlowControl|Sequence
    (:then_0
      (Utilities|FlowControl|Sequence
        (:then_0
          (Transformation|SetRelativeScale3D (Variables|Default|GetRoof) (Math|Vector|MakeVector (Variables|Properties|GetLength) (Variables|Properties|GetWidth) 0.0)))
        (:then_1
          (Transformation|SetRelativeScale3D (Variables|Default|GetFloor) (Math|Vector|MakeVector (Variables|Properties|GetLength) (Variables|Properties|GetWidth) 0.0))
          (Transformation|SetRelativeLocation (Variables|Default|GetFloor) (Math|Vector|MakeVector 0.0 0.0 (* (Variables|Properties|GetHeight) 1e+02)) false false))
        (:then_2
          (Transformation|SetRelativeScale3D (Variables|Default|GetFrontWall) (Math|Vector|MakeVector 0.0 (Variables|Properties|GetWidth) (Variables|Properties|GetHeight)))
          (Transformation|SetRelativeLocation (Variables|Default|GetFrontWall) (Math|Vector|MakeVector (* (Variables|Properties|GetLength) 5e+01) 0.0 (* (Variables|Properties|GetHeight) 5e+01)) false false))
        (:then_3
          (Transformation|SetRelativeScale3D (Variables|Default|GetBackWall) (Math|Vector|MakeVector 0.0 (Variables|Properties|GetWidth) (Variables|Properties|GetHeight)))
          (Transformation|SetRelativeLocation (Variables|Default|GetBackWall) (Math|Vector|MakeVector (* (Variables|Properties|GetLength) -5e+01) 0.0 (* (Variables|Properties|GetHeight) 5e+01)) false false))
        (:then_4
          (Transformation|SetRelativeScale3D (Variables|Default|GetRightWall) (Math|Vector|MakeVector (Variables|Properties|GetLength) 0.0 (Variables|Properties|GetHeight)))
          (Transformation|SetRelativeLocation (Variables|Default|GetRightWall) (Math|Vector|MakeVector 0.0 (* (Variables|Properties|GetWidth) 5e+01) (* (Variables|Properties|GetHeight) 5e+01)) false false))
        (:then_5
          (Transformation|SetRelativeScale3D (Variables|Default|GetLeftWall) (Math|Vector|MakeVector (Variables|Properties|GetLength) 0.0 (Variables|Properties|GetHeight)))
          (Transformation|SetRelativeLocation (Variables|Default|GetLeftWall) (Math|Vector|MakeVector 0.0 (* (Variables|Properties|GetWidth) -5e+01) (* (Variables|Properties|GetHeight) 5e+01)) false false))))
    (:then_1
      (Utilities|FlowControl|Sequence
        (:then_0
          (Rendering|Material|SetMaterial (Variables|Default|GetRoof) 0 (Variables|Material|GetMaterial)))
        (:then_1
          (Rendering|Material|SetMaterial (Variables|Default|GetFloor) 0 (Variables|Material|GetMaterial)))
        (:then_2
          (Rendering|Material|SetMaterial (Variables|Default|GetRightWall) 0 (Variables|Material|GetMaterial)))
        (:then_3
          (Rendering|Material|SetMaterial (Variables|Default|GetLeftWall) 0 (Variables|Material|GetMaterial)))
        (:then_4
          (Rendering|Material|SetMaterial (Variables|Default|GetFrontWall) 0 (Variables|Material|GetMaterial)))
        (:then_5
          (Rendering|Material|SetMaterial (Variables|Default|GetBackWall) 0 (Variables|Material|GetMaterial)))
        (:then_6
          (Transformation|SetRelativeLocation (Variables|Default|GetCenterObject) (Math|Vector|MakeVector 0.0 0.0 (+ (* (Variables|Properties|GetHeight) 5e+01) (Variables|Object|GetMeshOffset_Z))) false false))))))

(fn GetNextCamLocation
  (bind _result (Math|Integer|IncrementInt (Variables|Camera|Temp|GetCurrentCameraSelected))
    (:%20%20
      (if (> _result (select (Variables|Camera|Flags|GetbCurrentlyOnTop?) (- (Utilities|Array|Length (Variables|Camera|Temp|GetCameras)) 1) (- (Utilities|Array|Length (Variables|Camera|Temp|GetCameras)) 5)))
        (Variables|Camera|Temp|SetCurrentCameraSelected (select (Variables|Camera|Flags|GetbCurrentlyOnTop?) (Class|KismetSystemLibrary|MakeLiteralInteger 4) (Class|KismetSystemLibrary|MakeLiteralInteger))))
      (return (CallFunction|GetCurrentSelectedCamera)))))

(fn SpawnCamsAlongCorners
  (Utilities|Array|Clear (Variables|Camera|Temp|GetCameraPoints))
  (Utilities|Array|Clear (Variables|Camera|Temp|GetCameraPoints))
  (Utilities|FlowControl|Sequence
    (:then_0
      (Utilities|FlowControl|Sequence))
    (:then_1
      (if (not (Variables|Camera|Config|GetbOnlyTop))
        (Utilities|FlowControl|Sequence
          (:then_0
            (|SpawnCamera (* (Variables|Properties|GetLength) 5e+01) (* (Variables|Properties|GetWidth) 5e+01) (* (Variables|Properties|GetHeight) 0.0)))
          (:then_1)
          (:then_2)
          (:then_3))))))

(fn GetCurrentSelectedCamera
  (return (Utilities|Array|Get(acopy) (Variables|Camera|Temp|GetCameras) (Variables|Camera|Temp|GetCurrentCameraSelected))))

(fn ResetCam
  (Camera|SetFieldOfView (CallFunction|GetCurrentSelectedCamera) (Variables|Camera|Config|GetDefaultFOV)))

(fn ChangeLayer
  (if (not (Variables|Camera|Config|GetbOnlyTop))
    (if (Variables|Camera|Flags|GetbCurrentlyOnTop?)
      (Variables|Camera|Flags|SetbCurrentlyOnTop? false)
      (Variables|Camera|Temp|SetCurrentCameraSelected (- (Variables|Camera|Temp|GetCurrentCameraSelected) 4))
      (else
        (Variables|Camera|Flags|SetbCurrentlyOnTop? true)
        (Variables|Camera|Temp|SetCurrentCameraSelected (+ (Variables|Camera|Temp|GetCurrentCameraSelected) 4))))
    (return (CallFunction|GetCurrentSelectedCamera))
    (else
      (return (CallFunction|GetCurrentSelectedCamera)))))

(fn NextCamera
  (CallFunction|GetNextCamLocation)
  (return 0))

(fn ToggleLayer
  (CallFunction|ChangeLayer)
  (return 0))