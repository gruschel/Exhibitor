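; GM_Exhibitor is a spline test Blueprint that lays out two fixed hexagonal paths in its construction script.
; The script clears the ZRot and YRot splines, then adds six hardcoded local-space points to each.
; ZRot's points lie flat in the XY plane, while YRot's stand upright in the YZ plane, both starting at the origin.
; BeginPlay and Tick are empty, so nothing here moves along the splines.
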(event EventBeginPlay)

(event EventTick
  (params (DeltaSeconds :type Float%20%28single-precision%29)))

(fn ConstructionScript
  (Utilities|FlowControl|Sequence
    (:then_0
      (Spline|ClearSplinePoints (Variables|Default|GetZRot))
      (Utilities|FlowControl|Sequence
        (:then_0
          (Spline|AddSplinePoint (Variables|Default|GetZRot) (Math|Vector|MakeVector 0.0 0.0 0.0) "Local"))
        (:then_1
          (Spline|AddSplinePoint (Variables|Default|GetZRot) (Math|Vector|MakeVector 5e+01 -75.0 0.0) "Local"))
        (:then_2
          (Spline|AddSplinePoint (Variables|Default|GetZRot) (Math|Vector|MakeVector 1.5e+02 -75.0 0.0) "Local"))
        (:then_3
          (Spline|AddSplinePoint (Variables|Default|GetZRot) (Math|Vector|MakeVector 2e+02 0.0 0.0) "Local"))
        (:then_4
          (Spline|AddSplinePoint (Variables|Default|GetZRot) (Math|Vector|MakeVector 1.5e+02 75.0 0.0) "Local"))
        (:then_5
          (Spline|AddSplinePoint (Variables|Default|GetZRot) (Math|Vector|MakeVector 5e+01 75.0 0.0) "Local"))))
    (:then_1
      (Spline|ClearSplinePoints (Variables|Default|GetYRot))
      (Utilities|FlowControl|Sequence
        (:then_0
          (Spline|AddSplinePoint (Variables|Default|GetYRot) (Math|Vector|MakeVector 0.0 0.0 0.0) "Local"))
        (:then_1
          (Spline|AddSplinePoint (Variables|Default|GetYRot) (Math|Vector|MakeVector 0.0 -75.0 5e+01) "Local"))
        (:then_2
          (Spline|AddSplinePoint (Variables|Default|GetYRot) (Math|Vector|MakeVector 0.0 -75.0 1.5e+02) "Local"))
        (:then_3
          (Spline|AddSplinePoint (Variables|Default|GetYRot) (Math|Vector|MakeVector 0.0 0.0 2e+02) "Local"))
        (:then_4
          (Spline|AddSplinePoint (Variables|Default|GetYRot) (Math|Vector|MakeVector 0.0 75.0 1.5e+02) "Local"))
        (:then_5
          (Spline|AddSplinePoint (Variables|Default|GetYRot) (Math|Vector|MakeVector 0.0 75.0 5e+01) "Local"))))))